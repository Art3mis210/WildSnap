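; AggressiveAnimal is a hostile animal that chases the player and deals contact damage.
; When PawnSensing sees any pawn, it sets PlayerInSight, which is never cleared, and issues an AI move toward player character 0.
; Capsule hits against BP_FirstPersonCharacter call that character's TakeDamage with a fixed amount while the flag is set, with no cooldown between hits.
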(event `self.PawnSensing.OnSeePawn`
  (params (Pawn :type "Pawn Object Reference"))
  (set `self.PlayerInSight` true)
  (`self.FollowPlayer`))

(event `FollowPlayer`
  (if (`self.PlayerInSight`)
    (`|AIMoveTo` self (0.0 0.0 0.0) (`GameplayStatics.GetPlayerCharacter` 0) 10.0)))

(event `self.CapsuleComponent.OnComponentHit`
  (params (HitComponent :type "PrimitiveComponent Object Reference") (OtherActor :type "Actor Object Reference") (OtherComp :type "PrimitiveComponent Object Reference") (NormalImpulse :type "Vector Structure") (Hit :type "HitResult Structure (by ref)"))
  (bind _asbp_first_person_character (cast `/Game/Template/FirstPerson/Blueprints/BP_FirstPersonCharacter` OtherActor))
  (if (`self.PlayerInSight`)
    (`/Game/Template/FirstPerson/Blueprints/BP_FirstPersonCharacter.TakeDamage` _asbp_first_person_character 10.0)))

(fn `UserConstructionScript`)