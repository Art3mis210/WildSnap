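; Non-aggressive animal pawn that flees when it spots the player.
; Pawn sensing flags the player as nearby and sends the animal via AI MoveTo to a random navigable point within GetAwayDistance of itself, not specifically away from the player.
; Tick clears the nearby flag once the player is farther than GetAwayDistance, though the flag does not gate or repeat the movement.
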(event `self.PawnSensing.OnSeePawn`
  (params (Pawn :type "Pawn Object Reference"))
  (set `self.PlayerNearby` true)
  (`self.RunFromPlayer`))

(event `self.ReceiveTick`
  (params (DeltaSeconds :type "Float (single-precision)"))
  (if (`self.PlayerNearby`)
    (if (not (<= (`KismetMathLibrary.Vector_Distance` (`self.K2_GetActorLocation`) (`self.K2_GetActorLocation` (`GameplayStatics.GetPlayerCharacter` 0))) (`self.GetAwayDistance`)))
      (set `self.PlayerNearby` false))))

(event `RunFromPlayer`
  (`|AIMoveTo` self (`NavigationSystemV1.K2_GetRandomLocationInNavigableRadius` (`self.K2_GetActorLocation`) (`self.GetAwayDistance`) null null) null))

(fn `UserConstructionScript`)